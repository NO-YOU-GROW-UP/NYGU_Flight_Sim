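; PlanePawn_BP is a plane pawn that passes player axis input to its PlaneMovementComponent.
; Thrust, Pitch and Roll feed the component's throttle, pitch and roll inputs, and Thrust also prints the throttle percentage.
; BeginPlay activates the main Camera and deactivates ThirdPersonCamera.
; Leftover nodes for setting throttle, yaw input and a world offset are unconnected, so yaw has no control here.
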(event EventBeginPlay
  (Components|Activation|SetActive (Variables|Default|GetCamera) true true)
  (Components|Activation|SetActive (Variables|Default|GetThirdPersonCamera) false false))

(event Collision|EventActorBeginOverlap
  (params (OtherActor :type Actor%20Object%20Reference)))

(event EventTick
  (params (DeltaSeconds :type Float%20%28single-precision%29)))

(event Input|AxisEvents|InputAxisPitch
  (params (AxisValue :type Float%20%28single-precision%29))
  (Class|PlaneMovementComponent|AddPitchInput (Variables|Default|GetPlaneMovementComponent) AxisValue))

(event Input|AxisEvents|InputAxisThrust
  (params (AxisValue :type Float%20%28single-precision%29))
  (bind _planemovementcomponent (Variables|Default|GetPlaneMovementComponent))
  (Class|PlaneMovementComponent|AddThrottleInput _planemovementcomponent AxisValue)
  (Development|PrintString (Utilities|String|ToString(Float) (Variables|/Script/NYGU_Flight_Sim.PlaneMovementComponent|GetThrottlePercentage _planemovementcomponent))))

(event Input|AxisEvents|InputAxisRoll
  (params (AxisValue :type Float%20%28single-precision%29))
  (Class|PlaneMovementComponent|AddRollInput (Variables|Default|GetPlaneMovementComponent) AxisValue))

(event Input|KeyboardEvents|GenericUSBControllerButton1
  (params (Key :type Key%20Structure :default "None")))

(fn ConstructionScript)